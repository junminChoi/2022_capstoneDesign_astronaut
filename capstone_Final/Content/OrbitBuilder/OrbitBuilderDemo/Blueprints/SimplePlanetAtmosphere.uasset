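; SimplePlanetAtmosphere is an OrbitBuilder demo Blueprint for a planet with optional atmosphere and cloud layers.
; The construction script applies a configurable material to the Planet component.
; The HasAtmosphere and HasClouds flags decide whether the Athmosphere and Clouds components receive their materials or are destroyed.
; The event graph holds only disabled placeholder events, so the Blueprint adds no runtime logic.
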(event EventBeginPlay)

(event Collision|EventActorBeginOverlap
  (params (OtherActor :type Actor%20Object%20Reference)))

(event EventTick
  (params (DeltaSeconds :type Float%20%28single-precision%29)))

(fn ConstructionScript
  (Rendering|Material|SetMaterial (Variables|Default|GetPlanet) 0 (Variables|Default|GetMaterialPlanet))
  (if (Variables|Default|GetHasAtmosphere)
    (Rendering|Material|SetMaterial (Variables|Default|GetAthmosphere) 0 (Variables|Default|GetMaterialAtmosphere))
    (else
      (Components|DestroyComponent (Variables|Default|GetAthmosphere))))
  (if (Variables|Default|GetHasClouds)
    (Rendering|Material|SetMaterial (Variables|Default|GetClouds) 0 (Variables|Default|GetMaterialClouds))
    (else
      (Components|DestroyComponent (Variables|Default|GetClouds)))))