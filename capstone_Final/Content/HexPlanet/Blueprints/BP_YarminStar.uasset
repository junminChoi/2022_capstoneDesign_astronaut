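; BP_YarminStar is a pathfinding actor for the hex-tiled planet, with helper queries for hexagon location, continent, neighbors and faces.
; It caches BPHexPlanet's tile data, then finds routes by breadth-first search between hex indices or the hexes nearest two locations.
; Searches filter by continent type, optionally reject tiles via radial object traces, and bucket visited indices by hundreds.
; A Test event times a search and debug-draws the height-scaled path.
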(event Custom|Load
  (Variables|Default|SetLocal_Neighbors (Variables|/Game/HexPlanet/Blueprints/BP_HexPlanet_Moon.BP_HexPlanet_Moon_C|GetNeighborsIndexes (Variables|Default|GetBP_HexPlanet)))
  (Variables|Default|SetLocal_HexagonCenters (Variables|/Game/HexPlanet/Blueprints/BP_HexPlanet_Moon.BP_HexPlanet_Moon_C|GetHexagonCenterLocations (Variables|Default|GetBP_HexPlanet)))
  (Variables|Default|SetLocal_HexagonContinents (Variables|/Game/HexPlanet/Blueprints/BP_HexPlanet_Moon.BP_HexPlanet_Moon_C|GetHexagonsContinents (Variables|Default|GetBP_HexPlanet)))
  (Variables|Default|SetLocal_Continents (Variables|/Game/HexPlanet/Blueprints/BP_HexPlanet_Moon.BP_HexPlanet_Moon_C|GetContinentsParametrs (Variables|Default|GetBP_HexPlanet)))
  (Variables|Default|SetLocal_HexagonFaces (Variables|/Game/HexPlanet/Blueprints/BP_HexPlanet_Moon.BP_HexPlanet_Moon_C|GetCoordinatesMap (Variables|Default|GetBP_HexPlanet))))

(event Custom|Test
  (CallFunction|Load)
  (Variables|PathFinding|SetDateTime (Math|DateTime|UTCNow))
  (Rendering|Debug|FlushPersistentDebugLines)
  (bind (_issuccess _ispathfound _path_locations) (UserFunctions|PathFinding|FindPathLocation (Transformation|GetActorLocation) (Transformation|GetActorLocation (Variables|PathFinding|GetFindActor)) false "ObjectTypeQuery2" (Utilities|Array|MakeArray 0 1)))
  (Development|PrintString (Utilities|String|Append (Utilities|String|ToString(Float) (Class|KismetMathLibrary|GetTotalMilliseconds (- (Math|DateTime|UTCNow) (Variables|PathFinding|GetDateTime)))) " ms") true true "(R=1.000000,G=0.000000,B=0.013544,A=1.000000)" 1e+01)
  (if _ispathfound
    (for _array_element _path_locations
      (UserFunctions|LineTrace _array_element (Utilities|Array|MakeArray "ObjectTypeQuery1") "Persistent"))))

(event EventTick
  (params (DeltaSeconds :type Float%20%28single-precision%29)))

(event EventBeginPlay
  (Utilities|FlowControl|Delay 0.1)
  (CallFunction|Load))

(fn ConstructionScript)

(fn FindNearly2Vector
  (params (Array :type Array%20of%20Vectors) (StartLocation :type Vector) (EndLocation :type Vector))
  (for (_array_element _array_index) Array
    (Utilities|FlowControl|Sequence
      (:then_0
        (if (< (Math|Vector|VectorLength (- _array_element StartLocation)) (LocalVariables|GetL_Length))
          (LocalVariables|SetL_Length (Math|Vector|VectorLength (- _array_element StartLocation)))
          (LocalVariables|SetL_Key _array_index)
          (LocalVariables|SetL_Coord _array_element)))
      (:then_1
        (if (< (Math|Vector|VectorLength (- _array_element EndLocation)) (LocalVariables|GetL_Length_0))
          (LocalVariables|SetL_Length_0 (Math|Vector|VectorLength (- _array_element EndLocation)))
          (LocalVariables|SetL_Key_0 _array_index)
          (LocalVariables|SetL_Coord_0 _array_element)))))
  (return (LocalVariables|GetL_Key) (LocalVariables|GetL_Coord) (LocalVariables|GetL_Key_0) (LocalVariables|GetL_Coord_0)))

(fn LineTrace
  (params (Location :type Vector) (ObjectTypes :type Array%20of%20EObjectTypeQuery%20Enums :default "ObjectTypeQuery1") (DrawDebugType :type EDrawDebugTrace%20Enum :default "None"))
  (bind (_outhit _returnvalue) (Collision|LineTraceForObjects (+ Location (* (Math|Vector|Normalize Location 0.001) 1e+04)) (+ Location (* (Math|Vector|Normalize Location 0.001) -1e+04)) ObjectTypes false 0 DrawDebugType true "(R=0.000000,G=0.076761,B=1.000000,A=1.000000)" "(R=0.000000,G=1.000000,B=0.000000,A=1.000000)" 2e+01))
  (if _returnvalue
    (return true (.ImpactPoint (Collision|BreakHitResult _outhit)))
    (else
      (return false "0, 0, 0"))))

(fn FindPathLocation
  (params (StartLocation :type Vector) (EndLocation :type Vector) (IsExcludeObjectType :type Boolean) (ExludeObjectType :type EObjectTypeQuery%20Enum :default "ObjectTypeQuery1") (InclusiveContinent :type Array%20of%20Integers))
  (bind _l_startpoints_2 (LocalVariables|GetL_StartPoints_2))
  (LocalVariables|SetL_IsObjectType IsExcludeObjectType)
  (LocalVariables|SetL_StartLocation EndLocation)
  (LocalVariables|SetL_EndLocation StartLocation)
  (LocalVariables|SetL_ExcludeObjectType ExludeObjectType)
  (LocalVariables|SetL_InclusiveContinentType InclusiveContinent)
  (bind (_l_key1 _l_coord1 _l_key_01) (UserFunctions|FindNearly2Vector (Variables|Default|GetLocal_HexagonCenters) (LocalVariables|GetL_StartLocation) (LocalVariables|GetL_EndLocation)))
  (LocalVariables|SetL_StartPoint _l_key1)
  (LocalVariables|SetL_EndPoint _l_key_01)
  (if (Utilities|Array|ContainsItem (LocalVariables|GetL_InclusiveContinentType) (Utilities|Array|Get(acopy) (Variables|Default|GetLocal_HexagonContinents) (LocalVariables|GetL_StartPoint)))
    (if (Utilities|Array|ContainsItem (LocalVariables|GetL_InclusiveContinentType) (Utilities|Array|Get(acopy) (Variables|Default|GetLocal_HexagonContinents) (LocalVariables|GetL_EndPoint)))
      (Utilities|Array|Add (LocalVariables|GetL_StartPoints) (LocalVariables|GetL_StartPoint))
      (if (<= (Utilities|Array|Length (LocalVariables|GetL_StartPoints)) 0) :!label _label
        (return true false 0)
        (else
          (for _array_element (LocalVariables|GetL_StartPoints)
            (bind _output_get (LocalVariables|SetL_Neighbors_Cache (Utilities|Struct|BreakSMapInteger (Utilities|Array|Get(acopy) (Variables|Default|GetLocal_Neighbors) _array_element))))
            (for _array_element_2 _output_get
              (if (.ReturnValue (Utilities|Map|Find (LocalVariables|GetL_CheckedPoints) (/ _array_element_2 100)))
                (if (not (Utilities|Array|ContainsItem (Utilities|Struct|BreakSMapInteger (.Value (Utilities|Map|Find (LocalVariables|GetL_CheckedPoints) (/ _array_element_2 100)))) _array_element_2))
                  (if (== (LocalVariables|GetL_EndPoint) _array_element_2) :!label _label_2
                    (LocalVariables|SetL_PathFound true)
                    (Utilities|FlowControl|Sequence
                      (:then_0
                        (Utilities|FlowControl|Sequence :!label _label_3
                          (:then_0
                            (Utilities|Map|Add (LocalVariables|GetL_HexagonParents) _array_element_2 _array_element)
                            (Utilities|Array|Add (LocalVariables|GetL_StartPoints_2) _array_element_2))
                          (:then_1
                            (if (.ReturnValue (Utilities|Map|Find (LocalVariables|GetL_CheckedPoints) (/ _array_element_2 100))) :!label _label_4
                              (bind _output_get_2 (LocalVariables|SetL_CheckedPoint_Cache (Utilities|Struct|BreakSMapInteger (.Value (Utilities|Map|Find (LocalVariables|GetL_CheckedPoints) (/ _array_element_2 100))))))
                              (Utilities|Array|Add _output_get_2 _array_element_2)
                              (Utilities|Map|Add (LocalVariables|GetL_CheckedPoints) (/ _array_element_2 100) (Utilities|Struct|MakeSMapInteger _output_get_2))
                              (else
                                (Utilities|Map|Add (LocalVariables|GetL_CheckedPoints) (/ _array_element_2 100) (Utilities|Struct|MakeSMapInteger (Utilities|Array|MakeArray _array_element_2))))))))
                      (:then_1
                        (LocalVariables|SetL_Index _array_element_2)
                        (Utilities|Array|Add (LocalVariables|GetL_Path_Indexes) (LocalVariables|GetL_Index))
                        (Utilities|Array|Add (LocalVariables|GetL_Path_Locations) (* (Utilities|Array|Get(acopy) (Variables|Default|GetLocal_HexagonCenters) (LocalVariables|GetL_Index)) (.Height (Utilities|Struct|BreakSContenent (Utilities|Array|Get(acopy) (Variables|Default|GetLocal_Continents) (Utilities|Array|Get(acopy) (Variables|Default|GetLocal_HexagonContinents) (LocalVariables|GetL_Index)))))))
                        (if (== (.Value (Utilities|Map|Find (LocalVariables|GetL_HexagonParents) (LocalVariables|GetL_Index))) (LocalVariables|GetL_StartPoint)) :!label _label_5
                          (Utilities|Array|Add (LocalVariables|GetL_Path_Locations) (* (Utilities|Array|Get(acopy) (Variables|Default|GetLocal_HexagonCenters) (LocalVariables|GetL_StartPoint)) (.Height (Utilities|Struct|BreakSContenent (Utilities|Array|Get(acopy) (Variables|Default|GetLocal_Continents) (Utilities|Array|Get(acopy) (Variables|Default|GetLocal_HexagonContinents) (LocalVariables|GetL_StartPoint)))))))
                          (return true true (LocalVariables|GetL_Path_Locations))
                          (else
                            (bind _output_get_3 (LocalVariables|SetL_Index (.Value (Utilities|Map|Find (LocalVariables|GetL_HexagonParents) (LocalVariables|GetL_Index)))))
                            (Utilities|Array|Add (LocalVariables|GetL_Path_Indexes) _output_get_3)
                            (Utilities|Array|Add (LocalVariables|GetL_Path_Locations) (* (Utilities|Array|Get(acopy) (Variables|Default|GetLocal_HexagonCenters) (LocalVariables|GetL_Index)) (.Height (Utilities|Struct|BreakSContenent (Utilities|Array|Get(acopy) (Variables|Default|GetLocal_Continents) (Utilities|Array|Get(acopy) (Variables|Default|GetLocal_HexagonContinents) (LocalVariables|GetL_Index)))))))
                            (goto _label_5)))))
                    (elif (Utilities|Array|ContainsItem (LocalVariables|GetL_InclusiveContinentType) (Utilities|Array|Get(acopy) (Variables|Default|GetLocal_HexagonContinents) _array_element_2))
                      (if (LocalVariables|GetL_IsObjectType)
                        (bind _issuccess (UserFunctions|LineTrace (Utilities|Array|Get(acopy) (Variables|Default|GetLocal_HexagonCenters) _array_element_2) (Utilities|Array|MakeArray (LocalVariables|GetL_ExcludeObjectType)) "None"))
                        (if _issuccess
                          (goto _label_4)
                          (else
                            (goto _label_3)))
                        (else
                          (goto _label_3)))
                      (else
                        (goto _label_4)))))
                (else
                  (goto _label_2)))))
          (LocalVariables|SetL_StartPoints _l_startpoints_2)
          (Utilities|Array|Clear _l_startpoints_2)
          (goto _label)))
      (else
        (return false false 0)))
    (else
      (return false false 0))))

(fn FindPathPoints
  (params (StartPoint :type Integer) (EndPoint :type Integer) (IsExcludeObjectType :type Boolean) (ExludeObjectType :type EObjectTypeQuery%20Enum :default "ObjectTypeQuery1") (InclusiveContinent :type Array%20of%20Integers))
  (bind _l_startpoints_2 (LocalVariables|GetL_StartPoints_2))
  (LocalVariables|SetL_IsObjectType IsExcludeObjectType)
  (LocalVariables|SetL_StartPoint StartPoint)
  (LocalVariables|SetL_EndPoint EndPoint)
  (LocalVariables|SetL_ExcludeObjectType ExludeObjectType)
  (LocalVariables|SetL_InclusiveContinentType InclusiveContinent)
  (if (Utilities|Array|ContainsItem (LocalVariables|GetL_InclusiveContinentType) (Utilities|Array|Get(acopy) (Variables|Default|GetLocal_HexagonContinents) (LocalVariables|GetL_StartPoint)))
    (if (Utilities|Array|ContainsItem (LocalVariables|GetL_InclusiveContinentType) (Utilities|Array|Get(acopy) (Variables|Default|GetLocal_HexagonContinents) (LocalVariables|GetL_EndPoint)))
      (Utilities|Array|Add (LocalVariables|GetL_StartPoints) (LocalVariables|GetL_StartPoint))
      (if (<= (Utilities|Array|Length (LocalVariables|GetL_StartPoints)) 0) :!label _label
        (return true false 0)
        (else
          (for _array_element (LocalVariables|GetL_StartPoints)
            (bind _output_get (LocalVariables|SetL_Neighbors_Cache (Utilities|Struct|BreakSMapInteger (Utilities|Array|Get(acopy) (Variables|Default|GetLocal_Neighbors) _array_element))))
            (for _array_element_2 _output_get
              (if (.ReturnValue (Utilities|Map|Find (LocalVariables|GetL_CheckedPoints) (/ _array_element_2 100)))
                (if (not (Utilities|Array|ContainsItem (Utilities|Struct|BreakSMapInteger (.Value (Utilities|Map|Find (LocalVariables|GetL_CheckedPoints) (/ _array_element_2 100)))) _array_element_2))
                  (if (== (LocalVariables|GetL_EndPoint) _array_element_2) :!label _label_2
                    (LocalVariables|SetL_PathFound true)
                    (Utilities|FlowControl|Sequence
                      (:then_0
                        (Utilities|FlowControl|Sequence :!label _label_3
                          (:then_0
                            (Utilities|Map|Add (LocalVariables|GetL_HexagonParents) _array_element_2 _array_element)
                            (Utilities|Array|Add (LocalVariables|GetL_StartPoints_2) _array_element_2))
                          (:then_1
                            (if (.ReturnValue (Utilities|Map|Find (LocalVariables|GetL_CheckedPoints) (/ _array_element_2 100))) :!label _label_4
                              (bind _output_get_2 (LocalVariables|SetL_CheckedPoint_Cache (Utilities|Struct|BreakSMapInteger (.Value (Utilities|Map|Find (LocalVariables|GetL_CheckedPoints) (/ _array_element_2 100))))))
                              (Utilities|Array|Add _output_get_2 _array_element_2)
                              (Utilities|Map|Add (LocalVariables|GetL_CheckedPoints) (/ _array_element_2 100) (Utilities|Struct|MakeSMapInteger _output_get_2))
                              (else
                                (Utilities|Map|Add (LocalVariables|GetL_CheckedPoints) (/ _array_element_2 100) (Utilities|Struct|MakeSMapInteger (Utilities|Array|MakeArray _array_element_2))))))))
                      (:then_1
                        (LocalVariables|SetL_Index _array_element_2)
                        (Utilities|Array|Add (LocalVariables|GetL_Path_Indexes) (LocalVariables|GetL_Index))
                        (if (== (.Value (Utilities|Map|Find (LocalVariables|GetL_HexagonParents) (LocalVariables|GetL_Index))) (LocalVariables|GetL_StartPoint)) :!label _label_5
                          (return true true (LocalVariables|GetL_Path_Locations))
                          (else
                            (bind _output_get_3 (LocalVariables|SetL_Index (.Value (Utilities|Map|Find (LocalVariables|GetL_HexagonParents) (LocalVariables|GetL_Index)))))
                            (Utilities|Array|Add (LocalVariables|GetL_Path_Indexes) _output_get_3)
                            (Utilities|Array|Add (LocalVariables|GetL_Path_Locations) (* (Utilities|Array|Get(acopy) (Variables|Default|GetLocal_HexagonCenters) (LocalVariables|GetL_Index)) (.Height (Utilities|Struct|BreakSContenent (Utilities|Array|Get(acopy) (Variables|Default|GetLocal_Continents) (Utilities|Array|Get(acopy) (Variables|Default|GetLocal_HexagonContinents) (LocalVariables|GetL_Index)))))))
                            (goto _label_5)))))
                    (elif (Utilities|Array|ContainsItem (LocalVariables|GetL_InclusiveContinentType) (Utilities|Array|Get(acopy) (Variables|Default|GetLocal_HexagonContinents) _array_element_2))
                      (if (LocalVariables|GetL_IsObjectType)
                        (bind _issuccess (UserFunctions|LineTrace (Utilities|Array|Get(acopy) (Variables|Default|GetLocal_HexagonCenters) _array_element_2) (Utilities|Array|MakeArray (LocalVariables|GetL_ExcludeObjectType)) "None"))
                        (if _issuccess
                          (goto _label_4)
                          (else
                            (goto _label_3)))
                        (else
                          (goto _label_3)))
                      (else
                        (goto _label_4)))))
                (else
                  (goto _label_2)))))
          (LocalVariables|SetL_StartPoints _l_startpoints_2)
          (Utilities|Array|Clear _l_startpoints_2)
          (goto _label)))
      (else
        (return false false 0)))
    (else
      (return false false 0))))

(fn FindNearestHexagon
  (params (HexagonCenters :type Array%20of%20Vectors) (Location :type Vector))
  (for (_array_element _array_index) HexagonCenters
    (Utilities|FlowControl|Sequence
      (:then_0
        (if (< (Math|Vector|VectorLength (- _array_element Location)) (LocalVariables|GetL_Length))
          (LocalVariables|SetL_Length (Math|Vector|VectorLength (- _array_element Location)))
          (LocalVariables|SetL_Key _array_index)
          (LocalVariables|SetL_Coord _array_element)))))
  (return (LocalVariables|GetL_Key) (LocalVariables|GetL_Coord)))

(fn GetHexagonContinent
  (params (Index :type Integer))
  (bind _local_hexagoncontinents (Variables|Default|GetLocal_HexagonContinents))
  (bind _output (Utilities|Array|Get(acopy) _local_hexagoncontinents Index))
  (return _output (Utilities|Array|Get(acopy) (Variables|Default|GetLocal_Continents) _output)))

(fn GetHexagonLocation
  (params (Index :type Integer))
  (bind _local_hexagoncenters (Variables|Default|GetLocal_HexagonCenters))
  (bind _output (Utilities|Array|Get(acopy) _local_hexagoncenters Index))
  (return (* _output (.Height (Utilities|Struct|BreakSContenent (Utilities|Array|Get(acopy) (Variables|Default|GetLocal_Continents) (Utilities|Array|Get(acopy) (Variables|Default|GetLocal_HexagonContinents) Index))))) _output))

(fn GetHexagonFacesLocations
  (params (Index :type Integer))
  (bind _local_hexagoncontinents (Variables|Default|GetLocal_HexagonContinents))
  (bind _local_continents (Variables|Default|GetLocal_Continents))
  (bind _local_hexagonfaces (Variables|Default|GetLocal_HexagonFaces))
  (bind _output (Utilities|Array|Get(acopy) _local_hexagoncontinents Index))
  (bind _output_2 (Utilities|Array|Get(acopy) _local_hexagonfaces Index))
  (bind _vectors (Utilities|Struct|BreakSMapVector _output_2))
  (bind _output_3 (Utilities|Array|Get(acopy) _local_continents _output))
  (bind _height (Utilities|Struct|BreakSContenent _output_3))
  (bind _output_4 (Utilities|Array|Get(acopy) _vectors))
  (bind _output_get (LocalVariables|SetL_Array _vectors))
  (Utilities|Array|RemoveIndex _output_get)
  (bind _returnvalue (UserFunctions|ApplyVectorArray (LocalVariables|GetL_Array) _height false))
  (return (* _output_4 _height) _returnvalue _output_4 (LocalVariables|GetL_Array)))

(fn ApplyVectorArray
  (params (Array :type Array%20of%20Vectors) (Apply :type Float%20%28double-precision%29) (IsNormalize :type Boolean))
  (for _array_element Array
    (Utilities|Array|Add (LocalVariables|GetL_Vectors) (* (select IsNormalize (Math|Vector|Normalize _array_element) _array_element) Apply)))
  (return (LocalVariables|GetL_Vectors)))

(fn GetHexagonNeighbors
  (params (Index :type Integer))
  (return (Utilities|Struct|BreakSMapInteger (Utilities|Array|Get(acopy) (Variables|Default|GetLocal_Neighbors) Index))))

(fn CorrectPreDataPlanet
  (params (HexagonCenters :type Array%20of%20Vectors) (PlanetRotation :type Rotator) (PlanetLocation :type Vector))
  (for (_array_element _array_index) HexagonCenters
    (bind _continentparametrs (UserFunctions|GetHexagonContinent _array_index))
    (Utilities|Array|Add (LocalVariables|GetL_Array) (+ (Math|Vector|RotateVector (* _array_element (.Height (Utilities|Struct|BreakSContenent _continentparametrs))) PlanetRotation) PlanetLocation))
    (Utilities|Array|Add (LocalVariables|GetL_Array_0) (+ (Math|Vector|RotateVector _array_element PlanetRotation) PlanetLocation)))
  (return (LocalVariables|GetL_Array) (LocalVariables|GetL_Array_0)))