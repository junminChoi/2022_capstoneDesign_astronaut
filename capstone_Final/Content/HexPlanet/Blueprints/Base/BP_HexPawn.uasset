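; Player camera pawn for the hex planet that also handles selecting and commanding AI pawns.
; Axis input and mouse drag add zoom-scaled yaw and pitch with eased glide on release, while zoom interpolates spring arm length.
; A per-tick cursor trace places a decal and outlines mining actors or HISM instances.
; Left click selects an AI pawn; right click sends it to move or mine, swapping hovered instances for spawned BP_MiningActors.
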(event Custom|StopJumpMove
  ;[1 1 1] Movement
  ;;[1 1 1] Auto Interp
  (Utilities|FlowControl|Gate true) ; enters at Close
)

(event Custom|LineTrace
  (bind _returnvalue (Game|GetPlayerController 0))
  (bind _returnvalue_2 (Game|GetPlayerController 0))
  (bind _array (Utilities|Array|MakeArray "ObjectTypeQuery2" "ObjectTypeQuery1"))
  (bind _array_2 (Utilities|Array|MakeArray "ObjectTypeQuery1"))
  (bind _decal (Variables|Default|GetDecal))
  (bind _zoomclamp (Variables|Config|GetZoomClamp))
  (bind _hitresult (Class|PlayerController|GetHitResultUnderCursorforObjects _returnvalue _array_2 true))
  (bind (_hitresult_2 _returnvalue_3) (Class|PlayerController|GetHitResultUnderCursorforObjects _returnvalue_2 _array true))
  (bind (_x _y) (Math|Vector2D|BreakVector2D _zoomclamp))
  (bind (_bblockinghit _binitialoverlap _time _distance _location _impactpoint _normal _impactnormal) (Collision|BreakHitResult _hitresult))
  (bind (_bblockinghit_2 _binitialoverlap_2 _time_2 _distance_2 _location_2 _impactpoint_2 _normal_2 _impactnormal_2 _physmat _hitactor _hitcomponent _hitbonename _bonename _hititem) (Collision|BreakHitResult _hitresult_2))
  (Transformation|SetWorldLocationAndRotation _decal _location (Math|Rotator|MakeRotationfromAxes _impactnormal "0, 0, 0" "0, 0, 0") false false)
  (Transformation|SetWorldScale3D _decal (Math|Conversions|ToVector(Float) (Math|Float|MapRangeClamped (Variables|/Script/Engine.SpringArmComponent|GetTargetArmLength (Variables|Default|GetSpringArm)) _x _y 1.0 5.0)))
  (if _returnvalue_3
    (bind _asbp_mining_actor (Utilities|Casting|CastToBP_MiningActor _hitactor)
      (:then
        (if (!= (Variables|Default|GetHovered_MiningActor) _asbp_mining_actor)
          (bind _output_get (Variables|Default|SetHovered_MiningActor _asbp_mining_actor))
          (Rendering|SetRenderCustomDepth (Variables|/Game/HexPlanet/Blueprints/AIExample/BP_MiningActor.BP_MiningActor_C|GetStaticMesh _output_get) true)
          (Development|PrintString "Set Render Custom Depth")))
      (:CastFailed
        (Utilities|IsValid (Variables|Default|GetHovered_MiningActor)
          (:Is%20Valid
            (Rendering|SetRenderCustomDepth (Variables|/Game/HexPlanet/Blueprints/AIExample/BP_MiningActor.BP_MiningActor_C|GetStaticMesh (Variables|Default|GetHovered_MiningActor)) false)
            (Variables|Default|SetHovered_MiningActor 0))
          (:Is%20Not%20Valid
            _))
        (bind _as계층형_인스턴스드_스태틱_메시_컴포넌트 (Utilities|Casting|CastToHierarchicalInstancedStaticMeshComponent _hitcomponent)
          (:then
            (if (or (!= (Variables|Default|GetHovered_HISM) _as계층형_인스턴스드_스태틱_메시_컴포넌트) (!= _hititem (Variables|Default|GetHitItem)))
              (Variables|Default|SetHitItem _hititem)
              (Variables|Default|SetHovered_HISM _as계층형_인스턴스드_스태틱_메시_컴포넌트)
              (Rendering|SetVisibility (Variables|Default|GetOutline_StaticMesh) false false)
              (Transformation|SetWorldTransform (Variables|Default|GetOutline_StaticMesh) (Math|Transform|MakeTransform (.Location (Math|Transform|BreakTransform (.OutInstanceTransform (Components|InstancedStaticMesh|GetInstanceTransform _as계층형_인스턴스드_스태틱_메시_컴포넌트 (Variables|Default|GetHitItem) true)))) (.Rotation (Math|Transform|BreakTransform (.OutInstanceTransform (Components|InstancedStaticMesh|GetInstanceTransform _as계층형_인스턴스드_스태틱_메시_컴포넌트 (Variables|Default|GetHitItem) true)))) (* (.Scale (Math|Transform|BreakTransform (.OutInstanceTransform (Components|InstancedStaticMesh|GetInstanceTransform _as계층형_인스턴스드_스태틱_메시_컴포넌트 (Variables|Default|GetHitItem) true)))) 1.01)) false false)
              (Components|StaticMesh|SetStaticMesh (Variables|Default|GetOutline_StaticMesh) (Variables|/Script/Engine.StaticMeshComponent|GetStaticMesh _as계층형_인스턴스드_스태틱_메시_컴포넌트))
              (Rendering|SetVisibility (Variables|Default|GetOutline_StaticMesh) true false)
              (Development|PrintString (Utilities|String|ToString(Transform) (Math|Transform|MakeTransform (.Location (Math|Transform|BreakTransform (.OutInstanceTransform (Components|InstancedStaticMesh|GetInstanceTransform _as계층형_인스턴스드_스태틱_메시_컴포넌트 (Variables|Default|GetHitItem) true)))) (.Rotation (Math|Transform|BreakTransform (.OutInstanceTransform (Components|InstancedStaticMesh|GetInstanceTransform _as계층형_인스턴스드_스태틱_메시_컴포넌트 (Variables|Default|GetHitItem) true)))) (* (.Scale (Math|Transform|BreakTransform (.OutInstanceTransform (Components|InstancedStaticMesh|GetInstanceTransform _as계층형_인스턴스드_스태틱_메시_컴포넌트 (Variables|Default|GetHitItem) true)))) 1.01))))))
          (:CastFailed
            (Rendering|SetVisibility (Variables|Default|GetOutline_StaticMesh) false false)
            (Variables|Default|SetHitItem -1)
            (Variables|Default|SetHovered_HISM 0)))))))

(event Custom|DragMove_Tick2
  ;[1 1 1] Movement
  ;;[1 1 1] Auto Interp
  (Utilities|FlowControl|Gate true :!label _label
    (:Exit
      (if (not (Variables|Default|GetJumpInProgress))
        (bind _output_get (Variables|Default|SetCache (/ (Class|KismetMathLibrary|Vector2DInterpto :Current (* (Variables|Default|GetCache) 1e+01) :DeltaTime (Utilities|Time|GetWorldDeltaSeconds) :InterpSpeed 2.0) 1e+01)))
        (Pawn|Input|AddControllerYawInput (.X (Math|Vector2D|BreakVector2D _output_get)))
        (Pawn|Input|AddControllerPitchInput (.Y (Math|Vector2D|BreakVector2D _output_get)))
        (if (Class|KismetMathLibrary|IsNearlyZero2D (Variables|Default|GetCache) 0.001)
          (goto _label Close))))))

(event Custom|DragMove_Tick
  (bind _returnvalue (Game|GetPlayerController 0))
  (bind _zoomclamp (Variables|Config|GetZoomClamp))
  (bind (_deltax _deltay) (Class|PlayerController|GetInputMouseDelta _returnvalue))
  (bind (_x _y) (Math|Vector2D|BreakVector2D _zoomclamp))
  ;[1 1 1] Movement
  ;;[1 1 1] Drag Move
  (CallFunction|DragMoveTick2)
  (Utilities|FlowControl|Gate true
    (:Exit
      (bind _output_get (Variables|Default|SetCache (* (* (Math|Vector2D|MakeVector2D _deltax (* -1 _deltay)) (Variables|Config|GetDragMovementApply)) (Math|Float|MapRangeClamped (Variables|/Script/Engine.SpringArmComponent|GetTargetArmLength (Variables|Default|GetSpringArm)) _x _y 1.0 15.0))))
      (Pawn|Input|AddControllerYawInput (.X (Math|Vector2D|BreakVector2D _output_get)))
      (Pawn|Input|AddControllerPitchInput (.Y (Math|Vector2D|BreakVector2D _output_get))))))

(event Custom|Stop_DragMode
  ;[1 1 1] Movement
  ;;[1 1 1] Auto Interp
  (Utilities|FlowControl|Sequence
    (:then_0
      (Utilities|FlowControl|Gate true) ; enters at Open
    )))

(event EventBeginPlay
  (Variables|Default|SetZoomCache (Variables|/Script/Engine.SpringArmComponent|GetTargetArmLength (Variables|Default|GetSpringArm))))

(event EventTick
  (params (DeltaSeconds :type Float%20%28single-precision%29))
  (CallFunction|DragMoveTick)
  (CallFunction|LineTrace))

(event Input|ActionEvents|InputActionDragMove
  (params (Key :type Key%20Structure :default "None"))
  (bind _returnvalue (Game|GetPlayerController 0))
  (bind _returnvalue_2 (Game|GetPlayerController 0))
  (bind _zoomclamp (Variables|Config|GetZoomClamp))
  (bind (_deltax _deltay) (Class|PlayerController|GetInputMouseDelta _returnvalue))
  (bind (_x _y) (Math|Vector2D|BreakVector2D _zoomclamp))
  ;[1 1 1] Movement
  ;;[1 1 1] Drag Move
  (:Pressed
    (if (Variables|Default|GetAllowAnyCameraMovement)
      (CallFunction|StopJumpMove)
      (Variables|Default|SetEnableEdgeScrolling false)
      (Variables|/Script/Engine.PlayerController|SetbShowMouseCursor _returnvalue_2 true)
      (Input|SetInputModeGameOnly _returnvalue_2)
      (Utilities|FlowControl|Gate true) ; enters at Open
    ))
  (:Released
    (if (Variables|Default|GetAllowAnyCameraMovement)
      (CallFunction|StopDragMode)
      (Variables|Default|SetEnableEdgeScrolling true)
      (Variables|/Script/Engine.PlayerController|SetbShowMouseCursor _returnvalue_2 true)
      (Input|SetInputModeGameandUI _returnvalue_2 0 (CallFunction|MouseLocktoUI) true)
      (Utilities|FlowControl|Gate true) ; enters at Close
    )))

(event Input|AxisEvents|InputAxisMoveRight/Left
  (params (AxisValue :type Float%20%28single-precision%29))
  (bind _zoomclamp (Variables|Config|GetZoomClamp))
  (bind (_x _y) (Math|Vector2D|BreakVector2D _zoomclamp))
  ;[1 1 1] Movement
  ;;[1 1 1] Move Forwards and Sideways (Control top speeds in the MovementComponent)
  ;; Also absorbs edge scrolling
  (if (Variables|Default|GetAllowAnyCameraMovement)
    (switch Utilities|FlowControl|Switch|SwitchonEInputType (CallFunction|GetInputType)
      (:NewEnumerator0
        _)
      (:NewEnumerator1
        _))
    (if (or (> AxisValue 0.3) (< AxisValue -0.3))
      (Utilities|FlowControl|Sequence
        (:then_0
          (CallFunction|StopJumpMove)
          (bind _output_get (Variables|Default|SetCache (Math|Vector2D|MakeVector2D (* (* -1 AxisValue) (Variables|Config|GetMovementApply) (Math|Float|MapRangeClamped (Variables|/Script/Engine.SpringArmComponent|GetTargetArmLength (Variables|Default|GetSpringArm)) _x _y 1.0 15.0) 1.2) (.Y (Math|Vector2D|BreakVector2D (stale _output_get))))))
          (Pawn|Input|AddControllerYawInput (.X (Math|Vector2D|BreakVector2D _output_get))))
        (:then_1
          (goto _label Reset)))
      (else
        (Utilities|FlowControl|DoOnce false :!label _label
          (:Completed
            (CallFunction|StopDragMode)))))))

(event Input|AxisEvents|InputAxisMoveForward/Backward
  (params (AxisValue :type Float%20%28single-precision%29))
  (bind _zoomclamp (Variables|Config|GetZoomClamp))
  (bind (_x _y) (Math|Vector2D|BreakVector2D _zoomclamp))
  ;[1 1 1] Movement
  ;;[1 1 1] Move Forwards and Sideways (Control top speeds in the MovementComponent)
  ;; Also absorbs edge scrolling
  (if (Variables|Default|GetAllowAnyCameraMovement)
    (switch Utilities|FlowControl|Switch|SwitchonEInputType (CallFunction|GetInputType)
      (:NewEnumerator0
        _)
      (:NewEnumerator1
        _))
    (if (or (> AxisValue 0.3) (< AxisValue -0.3))
      (Utilities|FlowControl|Sequence
        (:then_0
          (CallFunction|StopJumpMove)
          (bind _output_get (Variables|Default|SetCache (Math|Vector2D|MakeVector2D (.X (Math|Vector2D|BreakVector2D (stale _output_get))) (* AxisValue (Variables|Config|GetMovementApply) (Math|Float|MapRangeClamped (Variables|/Script/Engine.SpringArmComponent|GetTargetArmLength (Variables|Default|GetSpringArm)) _x _y 1.0 15.0)))))
          (Pawn|Input|AddControllerPitchInput (.Y (Math|Vector2D|BreakVector2D _output_get))))
        (:then_1
          (goto _label Reset)))
      (else
        (Utilities|FlowControl|DoOnce false :!label _label
          (:Completed
            (CallFunction|StopDragMode)))))))

(event Input|AxisEvents|InputAxisZoom
  (params (AxisValue :type Float%20%28single-precision%29))
  (bind _zoomclamp (Variables|Config|GetZoomClamp))
  (bind (_x _y) (Math|Vector2D|BreakVector2D _zoomclamp))
  ;[1 1 1] Zoom
  (Variables|Default|SetZoomCache (Math|Float|Clamp(Float) (+ (Variables|Default|GetZoomCache) (* AxisValue (Variables|Config|GetZoomSpeed))) _x _y))
  (Variables|/Script/Engine.SpringArmComponent|SetTargetArmLength (Variables|Default|GetSpringArm) (Math|Interpolation|FInterpTo (Variables|/Script/Engine.SpringArmComponent|GetTargetArmLength (Variables|Default|GetSpringArm)) (Variables|Default|GetZoomCache) (Utilities|Time|GetWorldDeltaSeconds) 3.0)))

(event Input|MouseEvents|RightMouseButton
  (params (Key :type Key%20Structure :default "None"))
  (:Pressed
    (Utilities|IsValid (Variables|Default|GetSelected_AIPawn)
      (:Is%20Valid
        _)
      (:Is%20Not%20Valid
        (bind _outactors (Actor|GetAllActorsOfClass "/Game/HexPlanet/Blueprints/AIExample/BP_AIPawn.BP_AIPawn_C"))
        (Variables|Default|SetSelected_AIPawn (Utilities|Array|Get(acopy) _outactors))
        (Rendering|SetRenderCustomDepth (Variables|/Game/HexPlanet/Blueprints/AIExample/BP_AIPawn.BP_AIPawn_C|GetSkeletalMesh (Variables|Default|GetSelected_AIPawn)) true)))
    (Utilities|IsValid (Variables|Default|GetHovered_MiningActor)
      (:Is%20Valid
        (Default|FindPathMining (Variables|Default|GetSelected_AIPawn) (Variables|Default|GetHovered_MiningActor)))
      (:Is%20Not%20Valid
        (Utilities|IsValid (Variables|Default|GetHovered_HISM)
          (:Is%20Valid
            (bind _returnvalue (Game|SpawnActorfromClass "/Game/HexPlanet/Blueprints/AIExample/BP_MiningActor.BP_MiningActor_C" (.OutInstanceTransform (Components|InstancedStaticMesh|GetInstanceTransform (Variables|Default|GetHovered_HISM) (Variables|Default|GetHitItem) true)) "AlwaysSpawn" 0 0))
            (Default|SetNewMesh _returnvalue (Variables|/Script/Engine.StaticMeshComponent|GetStaticMesh (Variables|Default|GetHovered_HISM)))
            (Class|InstancedStaticMeshComponent|RemoveInstance (Variables|Default|GetHovered_HISM) (Variables|Default|GetHitItem))
            (Default|FindPathMining (Variables|Default|GetSelected_AIPawn) _returnvalue))
          (:Is%20Not%20Valid
            (Default|FindPathWithoutMining (Variables|Default|GetSelected_AIPawn) (.ImpactPoint (Collision|BreakHitResult (.HitResult (Class|PlayerController|GetHitResultUnderCursorforObjects (Game|GetPlayerController 0) (Utilities|Array|MakeArray "ObjectTypeQuery1") true)))))))))))

(event Input|MouseEvents|LeftMouseButton
  (params (Key :type Key%20Structure :default "None"))
  (bind _returnvalue (Game|GetPlayerController 0))
  (bind _array (Utilities|Array|MakeArray "ObjectTypeQuery3"))
  (bind (_hitresult _returnvalue_2) (Class|PlayerController|GetHitResultUnderCursorforObjects _returnvalue _array true))
  (:Pressed
    (if _returnvalue_2
      (bind _asbp_aipawn (Utilities|Casting|CastToBP_AIPawn (.HitActor (Collision|BreakHitResult _hitresult))))
      (Variables|Default|SetSelected_AIPawn _asbp_aipawn)
      (bind _outactors (Actor|GetAllActorsOfClass "/Game/HexPlanet/Blueprints/AIExample/BP_AIPawn.BP_AIPawn_C"))
      (for _array_element _outactors
        (Rendering|SetRenderCustomDepth (Variables|/Game/HexPlanet/Blueprints/AIExample/BP_AIPawn.BP_AIPawn_C|GetSkeletalMesh _array_element) false))
      (Rendering|SetRenderCustomDepth (Variables|/Game/HexPlanet/Blueprints/AIExample/BP_AIPawn.BP_AIPawn_C|GetSkeletalMesh (Variables|Default|GetSelected_AIPawn)) true))))

(fn ConstructionScript)

(fn GetYawRotation
  (params (Rotation :type Rotator))
  (return (Math|Rotator|MakeRotator 0.0 0.0 (.Yaw (Math|Rotator|BreakRotator Rotation)))))

(fn GetInputType
  (switch string (Game|GetPlatformName)
    (:IOS
      _)
    (:Android
      _)
    (:Windows
      (return "NewEnumerator0"))
    (:Mac
      (return "NewEnumerator0"))
    (:Linux
      (return "NewEnumerator0"))
    (:PS4
      (return "NewEnumerator1"))
    (:XboxOne
      (return "NewEnumerator1")))
  (return "NewEnumerator2"))

(fn MouseLocktoUI
  (return (select (Variables|Default|GetLockMouseToViewport) "LockAlways" "DoNotLock")))