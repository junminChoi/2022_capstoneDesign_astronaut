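; BP_MiningActor is a mineable object in the HexPlanet AI example that burns away once mined.
; MineFinished swaps the first two material slots to a burn dissolve material and sets IsMined.
; Tick then ramps the material's Lerp parameter over the dissolve duration and destroys the actor when the timer runs out.
; SetNewMesh allows the static mesh to be replaced.
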(event EventTick
  (params (DeltaSeconds :type Float%20%28single-precision%29))
  ;[1 1 1] When the object is mined, the dissolve effect begins
  (if (Variables|Default|GetIsMined)
    (bind _output_get (Variables|Default|SetTimer (+ (stale _output_get) DeltaSeconds)))
    (Rendering|Material|SetScalarParameterValueonMaterials (Variables|Default|GetStaticMesh) "Lerp" (Math|Float|MapRangeClamped _output_get 0.0 (Variables|Settings|GetDisolveEffectDurationSecond) 0.0 1.0))
    (if (>= (Variables|Default|GetTimer) (Variables|Settings|GetDisolveEffectDurationSecond))
      (Actor|DestroyActor))))

(fn ConstructionScript)

(fn SetNewMesh
  (params (NewMesh :type Static%20Mesh%20Object%20Reference))
  (Components|StaticMesh|SetStaticMesh (Variables|Default|GetStaticMesh) NewMesh))

(fn MineFinished
  (Rendering|Material|SetMaterial (Variables|Default|GetStaticMesh) 0 "/Game/HexPlanet/Materials/Dissolve/MI_BurnDissolveEffect.MI_BurnDissolveEffect")
  (Rendering|Material|SetMaterial (Variables|Default|GetStaticMesh) 1 "/Game/HexPlanet/Materials/Dissolve/MI_BurnDissolveEffect.MI_BurnDissolveEffect")
  (Variables|Default|SetIsMined true))