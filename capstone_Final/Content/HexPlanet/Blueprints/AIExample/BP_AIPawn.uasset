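; Example AI pawn that walks a spherical planet centered on the world origin and can mine target actors.
; FindPath requests a route from BP_YarminStar, draws it as debug points, then Tick steers through each point, keeping the pawn upright relative to the origin.
; On arrival, mining orders set the AnimBP flag, wait the target's duration, then call MineFinished.
; The construction script can optionally trace to snap and align it to the surface.
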(event Custom|StartMovement
  ;[1 1 1] Private Function
  (Variables|Default|SetIsStartMovement true)
  (Variables|Default|SetMovementIndex 1))

(event Custom|FindPath
  (params (EndLocation :type Vector))
  ;[1 1 1] FindPath
  (Variables|Default|SetIsStartMovement false)
  (bind (_issuccess _ispathfound _path_locations) (Default|FindPathLocation (Variables|Default|GetYarminStar) (Transformation|GetActorLocation) EndLocation true "ObjectTypeQuery2" (Utilities|Array|MakeArray 0)))
  (if _ispathfound
    (Variables|Default|SetMovementPath _path_locations)
    ;;[1 1 1] Debug Path
    (Rendering|Debug|FlushPersistentDebugLines)
    (for _array_element (Variables|Default|GetMovementPath)
      (Rendering|Debug|DrawDebugPoint _array_element 1e+01 "(R=0.000000,G=0.276817,B=1.000000,A=1.000000)" 1e+01))
    (CallFunction|StartMovement)
    (else
      (Development|PrintString "Path not found"))))

(event Custom|FindPath_Mining
  (params (MineActor :type BP%20Mining%20Actor%20Object%20Reference))
  ;[1 1 1] FindPath With Mining
  (bind _output_get (Variables|Default|SetMiningActor MineActor))
  (Variables|Default|SetIsMine true)
  (CallFunction|FindPath (Transformation|GetActorLocation _output_get)))

(event Custom|FindPath_WithoutMining
  (params (EndLocation :type Vector))
  ;[1 1 1] FindPath Without Mining
  (Variables|Default|SetIsMine false)
  (CallFunction|SetMiningAnimation false)
  (CallFunction|FindPath EndLocation))

(event Custom|MovementCompleted
  (bind _miningactor (Variables|Default|GetMiningActor))
  (Development|PrintString "Completed")
  ;[1 1 1] Mining After Movement Finished
  (if (Variables|Default|GetIsMine)
    (Utilities|IsValid (Variables|Default|GetMiningActor)
      (:Is%20Valid
        (CallFunction|SetMiningAnimation true)
        (Utilities|FlowControl|Delay (Variables|/Game/HexPlanet/Blueprints/AIExample/BP_MiningActor.BP_MiningActor_C|GetMiningDurationSeconds _miningactor))
        (if (Variables|Default|GetIsMine)
          (Default|MineFinished _miningactor)
          (CallFunction|SetMiningAnimation false))))))

(event EventBeginPlay
  ;[1 1 1] Initialization
  (bind _outactors (Actor|GetAllActorsOfClass "/Game/HexPlanet/Blueprints/BP_YarminStar.BP_YarminStar_C"))
  (Variables|Default|SetYarminStar (Utilities|Array|Get(acopy) _outactors)))

(event EventTick
  (params (DeltaSeconds :type Float%20%28single-precision%29))
  (bind _returnvalue (Math|Vector|MakeVector 0.0 0.0 0.0))
  (bind _returnvalue_2 (Transformation|GetActorLocation))
  (bind _returnvalue_3 (Math|Rotator|FindLookatRotation _returnvalue_2 _returnvalue))
  (bind (_roll _pitch _yaw) (Math|Rotator|BreakRotator _returnvalue_3))
  (if (Variables|Default|GetIsStartMovement)
    (Variables|Default|SetMovementLocation (Utilities|Array|Get(acopy) (Variables|Default|GetMovementPath) (Variables|Default|GetMovementIndex)))
    (if (Math|Vector|Equal(Vector) (Variables|Default|GetMovementLocation) (Transformation|GetActorLocation) 1.2e+02)
      ;[1 1 1] Movement Completed
      (bind _output_get (Variables|Default|SetMovementIndex (+ (stale _output_get) 1)))
      (if (> (Variables|Default|GetMovementIndex) (Utilities|Array|LastIndex (Variables|Default|GetMovementPath)))
        (Variables|Default|SetIsStartMovement false)
        (CallFunction|MovementCompleted))
      (else
        ;[1 1 1] Move To
        (Pawn|Input|AddMovementInput (Math|Rotator|GetRotationXVector (Math|Rotator|FindLookatRotation _returnvalue_2 (Variables|Default|GetMovementLocation))) 1.0 false)
        (Transformation|SetActorRotation (Math|Rotator|MakeRotator _roll (- _pitch -9e+01) _yaw))
        (Transformation|SetRelativeRotation (Variables|Default|GetSkeletalMesh) (Math|Rotator|MakeRotator 0.0 0.0 (+ (.Yaw (Math|Rotator|BreakRotator (Math|Transform|InverseTransformRotation (Transformation|GetWorldTransform (Variables|Default|GetScene)) (Math|Rotator|FindLookatRotation _returnvalue_2 (Variables|Default|GetMovementLocation))))) -9e+01)) false false)))))

(fn ConstructionScript
  (bind _returnvalue (Transformation|GetActorLocation))
  (if (Variables|Default|GetIsAutoAlighOnPlanet)
    (bind (_outhit _returnvalue_2) (Collision|LineTraceForObjects (+ _returnvalue (* (Math|Vector|Normalize _returnvalue 0.001) 1e+04)) (+ _returnvalue (* (Math|Vector|Normalize _returnvalue 0.001) -1e+04)) (Utilities|Array|MakeArray "ObjectTypeQuery1") false 0 "None"))
    (if _returnvalue_2
      (Transformation|SetActorLocationAndRotation (+ (.ImpactPoint (Collision|BreakHitResult _outhit)) (* (Math|Vector|Normalize (.ImpactPoint (Collision|BreakHitResult _outhit))) (Components|Capsule|GetScaledCapsuleHalfHeight (Variables|Default|GetCapsule)))) (Math|Rotator|MakeRotator (.Roll (Math|Rotator|BreakRotator (Math|Rotator|FindLookatRotation (.ImpactPoint (Collision|BreakHitResult _outhit)) (Math|Vector|MakeVector 0.0 0.0 0.0)))) (- (.Pitch (Math|Rotator|BreakRotator (Math|Rotator|FindLookatRotation (.ImpactPoint (Collision|BreakHitResult _outhit)) (Math|Vector|MakeVector 0.0 0.0 0.0)))) -9e+01) (.Yaw (Math|Rotator|BreakRotator (Math|Rotator|FindLookatRotation (.ImpactPoint (Collision|BreakHitResult _outhit)) (Math|Vector|MakeVector 0.0 0.0 0.0)))))))))

(fn SetMiningAnimation
  (params (IsMining :type Boolean))
  (bind _asthird_person_anim_bp (Utilities|Casting|CastToThirdPerson_AnimBP (Components|SkeletalMesh|GetAnimInstance (Variables|Default|GetSkeletalMesh))))
  (Variables|/Game/HexPlanet/EpicContent/Mannequin/Animations/ThirdPerson_AnimBP.ThirdPerson_AnimBP_C|SetIsMining _asthird_person_anim_bp IsMining))