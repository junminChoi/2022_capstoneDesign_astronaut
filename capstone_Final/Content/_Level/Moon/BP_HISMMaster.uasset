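; BP_HISMMaster is a central actor that pools static mesh placements into hierarchical instanced static mesh components, one per mesh.
; AddMesh looks up the mesh in HISMMap and adds a world-space instance, creating and registering a new component when none is valid.
; ClearInstances empties every mapped component and clears the map, but does not destroy the components.
; It has no active event logic, so other code must call these functions.
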(event EventBeginPlay)

(event Collision|EventActorBeginOverlap
  (params (OtherActor :type Actor%20Object%20Reference)))

(event EventTick
  (params (DeltaSeconds :type Float%20%28single-precision%29)))

(fn ConstructionScript)

(fn AddMesh
  (params (Key :type Static%20Mesh%20Object%20Reference%20%28by%20ref%29) (WorldTransform :type Transform%20%28by%20ref%29))
  (bind _hism_map (Variables|Default|GetHISM_Map))
  (bind (_value _returnvalue) (Utilities|Map|Find _hism_map Key))
  (if _returnvalue
    (Utilities|IsValid _value
      (:Is%20Valid
        (Class|InstancedStaticMeshComponent|AddInstanceWorldSpace _value WorldTransform))
      (:Is%20Not%20Valid
        (Utilities|Map|Remove _hism_map Key)
        (bind _returnvalue_2 (AddComponent|AddHierarchicalInstancedStaticMeshComponent false :!label _label))
        (Components|StaticMesh|SetStaticMesh _returnvalue_2 Key)
        (Class|InstancedStaticMeshComponent|AddInstanceWorldSpace _returnvalue_2 WorldTransform)
        (Utilities|Map|Add (Variables|Default|GetHISM_Map) Key _returnvalue_2)))
    (else
      (goto _label))))

(fn ClearInstances
  (bind _hism_map (Variables|Default|GetHISM_Map))
  (bind _values (Utilities|Map|Values _hism_map))
  (for _array_element _values
    (Components|InstancedStaticMesh|ClearInstances _array_element))
  (Utilities|Map|Clear _hism_map))