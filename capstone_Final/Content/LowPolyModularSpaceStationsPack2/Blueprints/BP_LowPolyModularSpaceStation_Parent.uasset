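; Parent Blueprint for modular low-poly space station pieces, exposing color, emissive and glass look settings on its base mesh.
; The construction script pushes emissive, glass and custom-color toggle parameters onto the mesh's materials.
; CustomColorFunction creates dynamic material instances for six material slots, sets a separate CustomColor on each, then reapplies emissive values.
; It has no runtime logic, as all event graph nodes are disabled.
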(event EventBeginPlay)

(event Collision|EventActorBeginOverlap
  (params (OtherActor :type Actor%20Object%20Reference)))

(event EventTick
  (params (DeltaSeconds :type Float%20%28single-precision%29)))

(fn ConstructionScript
  (bind _sm_basemesh (Variables|Default|GetSM_BaseMesh))
  (bind _sm_basemesh_2 (Variables|Default|GetSM_BaseMesh))
  (Utilities|FlowControl|Sequence
    (:then_0
      (Rendering|Material|SetScalarParameterValueonMaterials _sm_basemesh "EmissivePower" (Variables|Emissive|GetEmissivePower))
      (Rendering|Material|SetVectorParameterValueonMaterials _sm_basemesh "EmissiveColor" (Math|Conversions|ToVector(LinearColor) (Variables|Emissive|GetEmissiveColor))))
    (:then_2
      (CallFunction|CustomColorFunction (Variables|Default|GetSM_BaseMesh)))
    (:then_3
      (Rendering|Material|SetScalarParameterValueonMaterials (Variables|Default|GetSM_BaseMesh) "isCustomColors" (Math|Conversions|ToFloat(Boolean) (Variables|CustomColor|GetisCustomColors))))
    (:then_4
      (Rendering|Material|SetScalarParameterValueonMaterials _sm_basemesh_2 "GlassOpacity" (Variables|Glass|GetGlassOpacity))
      (Rendering|Material|SetVectorParameterValueonMaterials _sm_basemesh_2 "GlassColor" (Math|Conversions|ToVector(LinearColor) (Variables|Glass|GetGlassColor))))))

(fn CustomColorFunction
  (params (Target :type Mesh%20Component%20Object%20Reference))
  (Utilities|FlowControl|Sequence
    (:then_0
      (bind _returnvalue (Rendering|Material|CreateDynamicMaterialInstance Target 0 (Rendering|Material|GetMaterial Target 0) "None" :!class /Script/Engine.PrimitiveComponent))
      (Rendering|Material|SetVectorParameterValue _returnvalue "CustomColor" (Variables|CustomColor|GetColorMatID_00) :!class /Script/Engine.MaterialInstanceDynamic)
      (bind _returnvalue_2 (Rendering|Material|CreateDynamicMaterialInstance Target 1 (Rendering|Material|GetMaterial Target 1) "None" :!class /Script/Engine.PrimitiveComponent))
      (Rendering|Material|SetVectorParameterValue _returnvalue_2 "CustomColor" (Variables|CustomColor|GetColorMatID_01) :!class /Script/Engine.MaterialInstanceDynamic)
      (bind _returnvalue_3 (Rendering|Material|CreateDynamicMaterialInstance Target 2 (Rendering|Material|GetMaterial Target 2) "None" :!class /Script/Engine.PrimitiveComponent))
      (Rendering|Material|SetVectorParameterValue _returnvalue_3 "CustomColor" (Variables|CustomColor|GetColorMatID_02) :!class /Script/Engine.MaterialInstanceDynamic)
      (bind _returnvalue_4 (Rendering|Material|CreateDynamicMaterialInstance Target 3 (Rendering|Material|GetMaterial Target 3) "None" :!class /Script/Engine.PrimitiveComponent))
      (Rendering|Material|SetVectorParameterValue _returnvalue_4 "CustomColor" (Variables|CustomColor|GetColorMatID_03) :!class /Script/Engine.MaterialInstanceDynamic)
      (bind _returnvalue_5 (Rendering|Material|CreateDynamicMaterialInstance Target 4 (Rendering|Material|GetMaterial Target 4) "None" :!class /Script/Engine.PrimitiveComponent))
      (Rendering|Material|SetVectorParameterValue _returnvalue_5 "CustomColor" (Variables|CustomColor|GetColorMatID_04) :!class /Script/Engine.MaterialInstanceDynamic)
      (bind _returnvalue_6 (Rendering|Material|CreateDynamicMaterialInstance Target 5 (Rendering|Material|GetMaterial Target 5) "None" :!class /Script/Engine.PrimitiveComponent))
      (Rendering|Material|SetVectorParameterValue _returnvalue_6 "CustomColor" (Variables|CustomColor|GetColorMatID_05) :!class /Script/Engine.MaterialInstanceDynamic))
    (:then_1
      (Rendering|Material|SetScalarParameterValueonMaterials Target "EmissivePower" (Variables|Emissive|GetEmissivePower))
      (Rendering|Material|SetVectorParameterValueonMaterials Target "EmissiveColor" (Math|Conversions|ToVector(LinearColor) (Variables|Emissive|GetEmissiveColor))))))